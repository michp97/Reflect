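; Player pawn for grabbing, dragging and rotating movable components with the mouse, plus a Tab key that opens the pause menu and pauses the game.
; Right-click line-traces from the cursor, highlights the hit through custom depth stencil, and resets it to world origin if overlapping an actor.
; Tick moves the held component along the cursor ray at grab distance, flattened to Y=0, while the mouse wheel rotates it in fixed steps.
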(event EventBeginPlay
  (bind _returnvalue (Game|GetPlayerController 0))
  (Variables|/Script/Engine.PlayerController|SetbShowMouseCursor _returnvalue (not (Variables|/Script/Engine.PlayerController|GetbShowMouseCursor _returnvalue))))

(event EventTick
  (params (DeltaSeconds :type Float%20%28single-precision%29))
  (bind _returnvalue (Game|GetPlayerController 0))
  (bind _grabbedcomponent (Variables|Default|GetGrabbedComponent))
  (bind (_worldlocation _worlddirection) (Game|Player|ConvertMouseLocationToWorldSpace _returnvalue))
  (if (not (== _grabbedcomponent 0))
    (Transformation|SetWorldLocation _grabbedcomponent (* (Math|Transform|InverseTransformLocation (Math|Conversions|ToTransform(Vector) (Variables|Default|GetGrabLocation)) (+ _worldlocation (* _worlddirection (Variables|Default|GetDistance)))) "1.000000, 0,1.000000") false false)))

(event Input|KeyboardEvents|Tab
  (params (Key :type Key%20Structure :default "None"))
  (:Pressed
    (bind _returnvalue (UserInterface|CreateWidget "/Game/UI/PauseMenu.PauseMenu_C"))
    (bind _output_get (Variables|Default|SetMenuPauseWidget _returnvalue))
    (UserInterface|Viewport|AddtoViewport _output_get 0)
    (bind _aslevel_game_mode (Utilities|Casting|CastToLevelGameMode (Game|GetGameMode)))
    (bind _output_get_2 (Variables|/Script/cppProject.cppProjectGameModeBase|SetPaused _aslevel_game_mode true))
    (Game|SetGamePaused _output_get_2)))

(event Input|MouseEvents|RightMouseButton
  (params (Key :type Key%20Structure :default "None"))
  (bind _returnvalue (Game|GetPlayerController 0))
  (bind (_worldlocation _worlddirection) (Game|Player|ConvertMouseLocationToWorldSpace _returnvalue))
  (:Pressed
    (bind _outhit (Collision|LineTraceByChannel _worldlocation (+ _worldlocation (* _worlddirection (Math|Float|MakeLiteralFloat 1e+04))) "TraceTypeQuery4" true 0 "ForDuration"))
    (if (.bBlockingHit (Collision|BreakHitResult _outhit)) ; Hit?
      (bind _output_get (Variables|Default|SetGrabbedComponent (.HitComponent (Collision|BreakHitResult _outhit))))
      (Variables|Default|SetDistance (.Distance (Collision|BreakHitResult _outhit)))
      (if (== (Variables|/Script/Engine.SceneComponent|GetMobility (.HitComponent (Collision|BreakHitResult _outhit))) (Utilities|Enum|LiteralenumEComponentMobility "Movable")) ; Movable
        (Rendering|SetCustomDepthStencilValue _output_get 1)
        (Variables|Default|SetGrabLocation (- (.Location (Collision|BreakHitResult _outhit)) (Transformation|GetWorldLocation (Variables|Default|GetGrabbedComponent))))
        (for _array_element (Collision|GetOverlappingActors (Variables|Default|GetGrabbedComponent) "/Script/Engine.Actor" :!class /Script/Engine.PrimitiveComponent)
          (if (Collision|IsOverlappingActor (Variables|Default|GetGrabbedComponent) _array_element :!class /Script/Engine.PrimitiveComponent)
            (Transformation|SetWorldLocation (Variables|Default|GetGrabbedComponent) "0, 0, 0" false false)
            (Rendering|SetCustomDepthStencilValue (Variables|Default|GetGrabbedComponent) 0)))
        (else
          (Variables|Default|SetGrabbedComponent 0)))))
  (:Released
    (if (not (== (Variables|Default|GetGrabbedComponent) 0))
      (Rendering|SetCustomDepthStencilValue (Variables|Default|GetGrabbedComponent) 0)
      (Variables|Default|SetGrabbedComponent 0))))

(event Input|MouseEvents|MouseWheelUp
  (params (Key :type Key%20Structure :default "None"))
  (bind _grabbedcomponent (Variables|Default|GetGrabbedComponent))
  (:Pressed
    (if (== (Variables|/Script/Engine.SceneComponent|GetMobility (.HitComponent (Collision|BreakHitResult (stale Input|MouseEvents|RightMouseButton _outhit)))) (Utilities|Enum|LiteralenumEComponentMobility "Movable"))
      (Transformation|SetRelativeRotation _grabbedcomponent (Math|Rotator|CombineRotators (Variables|/Script/Engine.SceneComponent|GetRelativeRotation _grabbedcomponent) "5.000000, 0, 0") false false))))

(event Input|MouseEvents|MouseWheelDown
  (params (Key :type Key%20Structure :default "None"))
  (bind _grabbedcomponent (Variables|Default|GetGrabbedComponent))
  (:Pressed
    (if (== (Variables|/Script/Engine.SceneComponent|GetMobility (.HitComponent (Collision|BreakHitResult (stale Input|MouseEvents|RightMouseButton _outhit)))) (Utilities|Enum|LiteralenumEComponentMobility "Movable"))
      (Transformation|SetRelativeRotation _grabbedcomponent (Math|Rotator|CombineRotators (Variables|/Script/Engine.SceneComponent|GetRelativeRotation _grabbedcomponent) "-5.000000, 0, 0") true false))))

(fn ConstructionScript)