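; Laser emitter actor that fires a colored beam to activate sensors.
; Every Tick it calls CastLight from the arrow's location and forward direction, prints any hit sensor's signature, and calls Enable on it if already flagged Enabled, otherwise prints "Disabled".
; LaserColor tints the beam particles at construction, and the light and a dynamic emitter material at BeginPlay.
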(event EventBeginPlay
  (bind _lasercolor (Variables|Default|GetlaserColor))
  (Rendering|Components|Light|SetLightColor (Variables|Default|GetLight) _lasercolor true)
  (bind _returnvalue (Rendering|Material|CreateDynamicMaterialInstance (Variables|Default|GetmeshComp) 2 "/Game/Objects/Materials/emiter_light.emiter_light" "None" :!class /Script/Engine.PrimitiveComponent))
  (Rendering|Material|SetVectorParameterValue _returnvalue "BaseLight" _lasercolor :!class /Script/Engine.MaterialInstanceDynamic))

(event EventTick
  (params (DeltaSeconds :type Float%20%28single-precision%29))
  (bind _arrow (Variables|Default|GetArrow))
  (bind _output_get (Variables|Default|SethittedSensor (Class|LightEmiter|CastLight (Transformation|GetWorldLocation _arrow) (Math|Vector|GetForwardVector _arrow) (Variables|Default|GetcastDistance))))
  (if (not (== _output_get 0))
    (Development|PrintString (Variables|/Script/cppProject.LightSensor|GetSignature (Variables|Default|GethittedSensor)) true true "(R=1.000000,G=0.000000,B=0.000000,A=1.000000)")
    (if (Variables|/Script/cppProject.LightSensor|GetEnabled (Variables|Default|GethittedSensor))
      (Class|LightSensor|Enable (Variables|Default|GethittedSensor) true)
      (else
        (Development|PrintString "Disabled" true true "(R=0.771876,G=1.000000,B=0.000000,A=1.000000)")))))

(fn ConstructionScript
  (for _array_element (Variables|Default|GetPartArray)
    (Effects|Components|ParticleSystem|SetColorParameter _array_element "BeamColor" (Variables|Default|GetlaserColor))))