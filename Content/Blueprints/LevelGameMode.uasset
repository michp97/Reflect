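; Level game mode for a sensor-and-emitter puzzle that shows the game HUD, tracks completion and handles level loading.
; CompleteTask matches a trigger name's first character to the required sensors and stores that task's state.
; When all tasks pass, it calculates the score, then after a short delay shows the end screen and pauses.
; ReflectNr sums reflection counts once completion is reached, skipping consecutive repeats from one emitter.
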(event EventGo
  (params (Case :type Integer))
  (Viewport|RemoveAllWidgets)
  (Class|CppProjectGameModeBase|LoadLevel Case))

(event EventBeginPlay
  ;[1 1 1] Wyswietlanie HUDa gry
  (bind _returnvalue (UserInterface|CreateWidget "/Game/UI/GameHUD.GameHUD_C"))
  (UserInterface|Viewport|AddtoViewport _returnvalue 0))

(event EventReflectNr
  (params (Reflects :type Integer) (EmiterName :type String))
  (if (stale EventCompleteTask _returnvalue)
    (if (< (Variables|Default|Getiterator) (Utilities|Array|Length (Variables|Default|GetSensorsToComplete)))
      (if (not (Utilities|Enum|Equal(Enum) EmiterName (Variables|Default|GetCurrentEmiterName)))
        (Variables|Default|SetCurrentEmiterName EmiterName)
        (Variables|Default|Setiterator (+ (Variables|Default|Getiterator) 1))
        (bind _output_get (Variables|Default|SetCurrentReflectNumber (+ Reflects (Variables|Default|GetCurrentReflectNumber))))))))

(event EventCompleteTask
  (params (TriggerName :type String) (State :type Boolean))
  (for (_array_element _array_index) (Variables|Default|GetSensorsToComplete)
    (Development|PrintString _array_element)
    (if (Utilities|Enum|Equal(Enum) _array_element (Class|KismetStringLibrary|Mid TriggerName 0 1))
      (Utilities|Array|SetArrayElem (Variables|Default|GetCompletedTasks) _array_index State)
      (Development|PrintString _array_element true true "(R=1.000000,G=1.000000,B=1.000000,A=1.000000)")
      (bind _returnvalue (Class|CppProjectGameModeBase|CheckTask))
      (if _returnvalue
        (bind _returnvalue_2 (Game|GetCurrentLevelName true))
        (bind _returnvalue_3 (Class|CppProjectGameModeBase|CalculateScore))
        (Utilities|FlowControl|Delay 1.0)
        (bind _returnvalue_4 (UserInterface|CreateWidget "/Game/UI/EndLevelScreen.EndLevelScreen_C"))
        (bind _output_get (Variables|Default|SetEndScreenWidget _returnvalue_4))
        (UserInterface|Viewport|AddtoViewport _output_get 0)
        (Class|CppProjectGameModeBase|PauseGame true)))))

(event EventTick
  (params (DeltaSeconds :type Float%20%28single-precision%29)))

(fn ConstructionScript)